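; Base weapon actor that fires projectiles automatically while the trigger is held.
; PullTrigger fires once immediately, then starts a looping timer on Fire at the RoundsPerSecond rate, gated by a DoOnce against repeated pulls.
; ReleaseTrigger clears that timer and resets the DoOnce.
; Each Fire spawns the Projectile class at the ProjectileSpawnPoint component's world transform.
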(event Custom|PullTrigger
  (Utilities|FlowControl|DoOnce false
    (:Completed
      (CallFunction|Fire)
      (Utilities|Time|SetTimerbyFunctionName 0 "Fire" (/ 1.0 (Variables|Default|GetRounds%20per%20second)) true))))

(event Custom|ReleaseTrigger
  (Utilities|Time|ClearTimerbyFunctionName 0 "Fire")
  (Utilities|FlowControl|DoOnce false) ; enters at Reset
)

(event Custom|Fire
  (Game|SpawnActorfromClass "/Game/Blueprints/Projectile.Projectile_C" (Transformation|GetWorldTransform (Variables|Default|GetProjectileSpawnPoint)) "Undefined" 0 0))

(event EventBeginPlay)

(event Collision|EventActorBeginOverlap
  (params (OtherActor :type Actor%20Object%20Reference)))

(event EventTick
  (params (DeltaSeconds :type Float%20%28single-precision%29)))

(fn ConstructionScript)